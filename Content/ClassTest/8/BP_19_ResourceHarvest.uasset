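; Test actor for a resource harvesting mechanic with a timed gather boost.
; BeginPlay enables player input and starts a looping one-second timer that calls AddResources.
; AddResources sets ResourceCount to the boosted or normal gather rate, overwriting rather than accumulating it, and prints it for one frame's delta time.
; ActivateBoost, also triggered by the B key, sets IsBoosted, then clears it after BoostDuration, printing both changes.
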(event `self.ReceiveBeginPlay`
  (`self.EnableInput` (`GameplayStatics.GetPlayerController` 0))
  (`KismetSystemLibrary.K2_SetTimer` null "AddResources" 1.0 true))

(event `AddResources`
  ;[0 0.005169 0.15 0.5] Gather Rate
  (if (`self.bIsBoosted`)
    (set `self.ResourceCount` (+ (`self.GatherRateBoosted`) 0))
    (`KismetSystemLibrary.PrintString` (`KismetStringLibrary.Concat_StrStr` "Amount of Resource's: " (`KismetStringLibrary.Conv_IntToString` (`self.ResourceCount`))) true true (struct :`G` 0.66 :`B` 1.0 :`A` 1.0) (`GameplayStatics.GetWorldDeltaSeconds`))
    (else
      (set `self.ResourceCount` (+ 0 (`self.GatherRateNormal`)))
      (`KismetSystemLibrary.PrintString` (`KismetStringLibrary.Concat_StrStr` "Amount of Resource's: " (`KismetStringLibrary.Conv_IntToString` (`self.ResourceCount`))) true true (struct :`G` 0.66 :`B` 1.0 :`A` 1.0) (`GameplayStatics.GetWorldDeltaSeconds`)))))

(event `ActivateBoost`
  ;[0.02201 0.15 0 0.5] Activate Boost
  (set `self.bIsBoosted` true :!label _label)
  (`KismetSystemLibrary.PrintString` "Boost activated!")
  (`KismetSystemLibrary.Delay` (`self.BoostDuration`))
  (set `self.bIsBoosted` false)
  (`KismetSystemLibrary.PrintString` "Boost Deactivating!"))

(event `Key|B`
  (params (Key :type "Key Structure"))
  ;[0.02201 0.15 0 0.5] Activate Boost
  (:`Pressed`
    (goto _label)))

(fn `UserConstructionScript`)