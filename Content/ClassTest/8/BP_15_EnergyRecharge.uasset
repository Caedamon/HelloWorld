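; Class-test Blueprint that prototypes an energy recharge, reporting its state through printed messages.
; BeginPlay starts a one-second looping timer with no function name shown and calls RechargeEnergy, which adds RechargeRate to CurrentEnergy, clamped to MaxEnergy.
; After a delay it calls RechargeTrigger, which at zero energy only toggles RechargePaused around another delay and prints messages.
; RechargePaused is set true immediately before its check, so it never blocks recharging.
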(event `RechargeEnergy`
  ;[0.006344 0.15 0 0.5] Recharge?
  (bind _output_get (set `self.bRechargePaused` true))
  (if _output_get
    (set `self.CurrentEnergy` (`KismetMathLibrary.FClamp` (+ (`self.RechargeRate`) (`self.CurrentEnergy`)) 0.0 (`self.MaxEnergy`)))
    (`KismetSystemLibrary.PrintString` "Your Energy has been Recharged!")
    (`KismetSystemLibrary.Delay` 5.0)
    (`self.RechargeTrigger`)))

(event `self.ReceiveBeginPlay`
  (`KismetSystemLibrary.K2_SetTimer` null "" 1.0 true)
  (`self.RechargeEnergy`))

(event `RechargeTrigger`
  ;[0.1295 0 0.15 0.5] If nrg = 0, start recharging... i think xD'
  (if (<= (`self.CurrentEnergy`) 0.0)
    (`KismetSystemLibrary.PrintString` "Out of Energy!")
    (set `self.bRechargePaused` false)
    (`KismetSystemLibrary.Delay` 5.0)
    (set `self.bRechargePaused` true)
    (`KismetSystemLibrary.PrintString` "Energy Recharging")))

(fn `UserConstructionScript`)