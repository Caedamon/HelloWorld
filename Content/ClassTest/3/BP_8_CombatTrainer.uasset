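; BP_8_CombatTrainer is a class-test Blueprint that demonstrates basic combat math by printing results at startup.
; BeginPlay uses a Sequence to fire five custom events for health pickup, damage, critical hit, ammo clips and final score.
; Each event computes from member variables, stores the result in a separate variable and prints it with a label.
; Only the health pickup clamps its result.
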(event `CustomEvent_AddHealth`
  ;[0 0.15 0.005689 0.5] Health Pickup
  (bind _output_get (set `self.ClampedHealth,` (`KismetMathLibrary.FClamp` (+ (`self.HealthPack`) (`self.CurrentHealth`)) 0.0 100.0)))
  (`KismetSystemLibrary.PrintString` (`KismetStringLibrary.Concat_StrStr` "Health: " (`KismetStringLibrary.Conv_DoubleToString` _output_get)) true true (struct :`G` 1.0 :`B` 0.044867 :`A` 1.0)))

(event `CustomEvent_CalculateDamage`
  ;[0.15 0 0.01502 0.5] Damage Method
  (bind _output_get (set `self.NewHealth` (`KismetMathLibrary.Conv_IntToDouble` (- (`self.PlayerHealth`) (`self.DamageTaken`)))))
  (`KismetSystemLibrary.PrintString` (`KismetStringLibrary.Concat_StrStr` "Health: " (`KismetStringLibrary.Conv_DoubleToString` _output_get)) true true (struct :`R` 0.611 :`A` 1.0)))

(event `CustomEvent_CriticalHit`
  ;[0.15 0 0.1137 0.5] CRIT HIT!
  (bind _output_get (set `self.CritDamage,` (* (`self.BaseDamage`) (`self.CritMultiplier`))))
  (`KismetSystemLibrary.PrintString` (`KismetStringLibrary.Concat_StrStr` "CRITTICAL HIT!: " (`KismetStringLibrary.Conv_DoubleToString` _output_get))))

(event `self.ReceiveBeginPlay`
  ; If you turn this on its side it looks like a chandaleir!
  (`|ExecutionSequence`
    (:`then_0`
      (`self.CustomEvent_AddHealth`))
    (:`then_1`
      (`self.CustomEvent_CalculateDamage`))
    (:`then_2`
      (`self.CustomEvent_CriticalHit`))
    (:`then_3`
      (`self.CustomEvent_AmmoStatus`))
    (:`then_4`
      (`self.CustomEvent_UpdateScore`))))

(event `CustomEvent_AmmoStatus`
  ;[0 0.08461 0.15 0.5] Ammo Clip Counter
  (bind _output_get (set `self.ClipsRemaining` (/ (`self.ReserveAmmo`) (`self.ClipSize`))))
  (`KismetSystemLibrary.PrintString` (`KismetStringLibrary.Concat_StrStr` (`KismetStringLibrary.Conv_IntToString` _output_get) " Clips Remaining: ")))

(event `CustomEvent_UpdateScore`
  ;[0.4233 1 0.8071 0.5] Score Counter
  (bind _output_get (set `self.UpdatedScore` (- (* (+ (`self.BaseScore`) (`self.StreakBonus`)) (`self.ComboMult`)) (`self.Penalty`))))
  (`KismetSystemLibrary.PrintString` (`KismetStringLibrary.Concat_StrStr` "Final Score!: " (`KismetStringLibrary.Conv_DoubleToString` _output_get))))

(fn `UserConstructionScript`)