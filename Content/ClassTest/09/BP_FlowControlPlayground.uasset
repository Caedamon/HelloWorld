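; Test playground Blueprint that demonstrates flow control nodes through printed messages.
; BeginPlay enables input, and keys 1–8 call labs for DoOnce, counter-based DoN, Sequence, loops, MultiGate, FlipFlop and Gate.
; R triggers the DoOnce MultiInput reset, W resets the MultiGate, and O and C open or close the Gate.
; The lab chains into the DoOnce MultiInput inputs are never executed.
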(event `ResetDoOnce_Lab`
  ;[0.1147 0.15 0 0.5] MultiInput Function to run each lab.
  (`|DoOnceMultiInput` :!via `Reset In` :!label _label
    (:`A Out`
      (set `self.CurrentStrikes` 0))
    (:`Reset Out`
      (`KismetSystemLibrary.PrintString` "Resetting!"))))

(event `Key|R`
  (params (Key :type "Key Structure"))
  ;[0.1147 0.15 0 0.5] MultiInput Function to run each lab.
  (:`Pressed`
    (goto _label :!via `Reset In`)))

(event `self.ReceiveBeginPlay`
  (`self.EnableInput` (`GameplayStatics.GetPlayerController` 0)))

(event `DoOnce_Lab`
  ;[0.01255 0 0.15 0.5] DoOnce
  (`/Engine/EditorBlueprintResources/StandardMacros.DoOnce` false
    (:`Completed`
      (`KismetSystemLibrary.PrintString` "Hello Unreal World... or something!"))))

(event `DoN_Lab`
  ;[0 0.04727 0.15 0.5] DoN
  (if (< (`self.CurrentStrikes`) (`self.StrikeLimit`))
    (bind _result (`/Engine/EditorBlueprintResources/StandardMacros.IncrementInt` (`self.CurrentStrikes`))
      (:`  `
        (set `self.CurrentStrikes` _result)
        (`KismetSystemLibrary.PrintString` (`KismetStringLibrary.Concat_StrStr` "Current Strikes: " (`KismetStringLibrary.Conv_IntToString` (`self.CurrentStrikes`))))))))

(event `ResetDoN_Lab`
  ;[0 0.04727 0.15 0.5] DoN
  (set `self.CurrentStrikes` 0))

(event `Key|One`
  (params (Key :type "Key Structure"))
  (:`Released`
    (`self.DoOnce_Lab`)))

(event `Sequence_Lab`
  ;[0 0.07631 0.15 0.5] Sequencer
  (`|ExecutionSequence`
    (:`then_0`
      (`KismetSystemLibrary.PrintString` "Ready!"))
    (:`then_1`
      (`KismetSystemLibrary.PrintString` "Set!"))
    (:`then_2`
      (`KismetSystemLibrary.PrintString` "Go!"))))

(event `Key|Two`
  (params (Key :type "Key Structure"))
  (:`Released`
    (`self.DoN_Lab`)))

(event `ForLoop_Lab`
  ;[0 0.1199 0.15 0.5] For Loop
  (for _index (range 5)
    (`KismetSystemLibrary.PrintString` (`KismetStringLibrary.Concat_StrStr` "Index is: " (`KismetStringLibrary.Conv_IntToString` _index)))))

(event `Key|Three`
  (params (Key :type "Key Structure"))
  (:`Released`
    (`self.Sequence_Lab`)))

(event `Key|Four`
  (params (Key :type "Key Structure"))
  (:`Released`
    (`self.WhileLoop_Lab`)))

(event `Key|Five`
  (params (Key :type "Key Structure"))
  (:`Released`
    (`self.ForLoop_Lab`)))

(event `Key|Six`
  (params (Key :type "Key Structure"))
  (:`Released`
    (`self.Multigate_Lab`)))

(event `WhileLoop_Lab`
  ;[0 0.15 0.1152 0.5] While Loop
  (while (< (`self.GoalCount`) 3)
    (`KismetSystemLibrary.PrintString` (`KismetStringLibrary.Concat_StrStr` "Not There yet!" " Adding One!"))
    (bind _result (`/Engine/EditorBlueprintResources/StandardMacros.IncrementInt` (`self.GoalCount`))
      (:`  `
        (set `self.GoalCount` _result))))
  (`KismetSystemLibrary.PrintString` "Goal Reached!!!"))

(event `Multigate_Lab`
  ;[0.15 0 0.007461 0.5] ED-209
  (`|MultiGate` false :!label _label_2
    (:`Out 0`
      (`KismetSystemLibrary.PrintString` "Weapon Detected!"))
    (:`Out 1`
      (`KismetSystemLibrary.PrintString` "Drop your weapon! you have 15 seconds to comply!"))
    (:`Out 2`
      (`KismetSystemLibrary.PrintString` "Error: Weapon Routine Malfunction, Resetting in 3, 2, 1...."))))

(event `Key|W`
  (params (Key :type "Key Structure"))
  ;[0.15 0 0.007461 0.5] ED-209
  (:`Pressed`
    (goto _label_2 :!via `Reset`)))

(event `Key|Seven`
  (params (Key :type "Key Structure"))
  (:`Released`
    (`self.FlipFlop_Lab`)))

(event `Key|Eight`
  (params (Key :type "Key Structure"))
  (:`Released`
    (`self.Gate_Lab`)))

(event `FlipFlop_Lab`
  ;[0 0.15 0.02018 0.5] Flipflop
  (`KismetSystemLibrary.PrintString` "Fliping the Flop!")
  (`/Engine/EditorBlueprintResources/StandardMacros.FlipFlop`
    (:`A`
      (`KismetSystemLibrary.PrintString` "The Flop has Been Flipped!"))
    (:`B`
      (`KismetSystemLibrary.PrintString` "The Flip has been Flopped!"))))

(event `Gate_Lab`
  ;[0.01633 0.15 0 0.5] Gate
  (`/Engine/EditorBlueprintResources/StandardMacros.Gate` true :!label _label_3
    (:`Exit`
      (`KismetSystemLibrary.PrintString` "Access Granted! ENGAGING!"))))

(event `Key|O`
  (params (Key :type "Key Structure"))
  ;[0.01633 0.15 0 0.5] Gate
  (:`Pressed`
    (goto _label_3 :!via `Open`)))

(event `Key|C`
  (params (Key :type "Key Structure"))
  ;[0.01633 0.15 0 0.5] Gate
  (:`Pressed`
    (goto _label_3 :!via `Close`)))

(fn `UserConstructionScript`)