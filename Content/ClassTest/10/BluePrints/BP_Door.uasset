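; BP_Door is a hinged door that the player toggles with E, with input enabled while overlapping its trigger.
; While IsOpen, Tick swings DoorPivot toward -90 yaw through RotateDoorByYaw, a frame-rate-scaled helper, and calls AutoClose.
; After five seconds, AutoClose applies only one closing rotation step and clears IsOpen, so the door does not swing shut.
; An uncalled backup event holds continuous open/close logic.
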(event `DoorOpenOnTick`
  (bind (_relativerotation_roll _relativerotation_pitch _relativerotation_yaw) (`KismetMathLibrary.BreakRotator` (`SceneComponent.RelativeRotation` (`self.DoorPivot`))))
  ;[0.01756 0.15 0 0.5] Open Door on Tick
  (if (`self.bIsOpen`)
    (if (>= _relativerotation_yaw -90.0)
      (`self.RotateDoorByYaw` 100.0 -1.0)
      (`self.AutoClose`))))

(event `OpenDoorTickBackup`
  (bind (_relativerotation_roll _relativerotation_pitch _relativerotation_yaw) (`KismetMathLibrary.BreakRotator` (`SceneComponent.RelativeRotation` (`self.DoorPivot`))))
  (bind (_relativerotation_roll_2 _relativerotation_pitch_2 _relativerotation_yaw_2) (`KismetMathLibrary.BreakRotator` (`SceneComponent.RelativeRotation` (`self.DoorPivot`))))
  ; OpenDoor on Tick Origin Backup
  (if (`self.bIsOpen`)
    (if (> _relativerotation_yaw -90.0)
      (`SceneComponent.K2_AddRelativeRotation` (`self.DoorPivot`) (`KismetMathLibrary.MakeRotator` 0.0 0.0 (* (`GameplayStatics.GetWorldDeltaSeconds`) -100.0)) false false))
    (elif (< _relativerotation_yaw_2 0.0)
      (`SceneComponent.K2_AddRelativeRotation` (`self.DoorPivot`) (`KismetMathLibrary.MakeRotator` 0.0 0.0 (* (`GameplayStatics.GetWorldDeltaSeconds`) 100.0)) false false))))

(event `AutoClose`
  (bind (_relativerotation_roll _relativerotation_pitch _relativerotation_yaw) (`KismetMathLibrary.BreakRotator` (`SceneComponent.RelativeRotation` (`self.DoorPivot`))))
  ;[0.15 0.002581 0 0.5] AutoClose Door
  (if (`self.bIsOpen`)
    (`KismetSystemLibrary.Delay` 5.0)
    (if (<= _relativerotation_yaw 0.0)
      (`self.RotateDoorByYaw` 100.0)
      (set `self.bIsOpen` false))))

(event `self.ReceiveTick`
  (params (DeltaSeconds :type "Float (single-precision)"))
  (`self.DoorOpenOnTick`))

(event `self.PlayerOverlappDoor.OnComponentBeginOverlap`
  (params (OverlappedComponent :type "PrimitiveComponent Object Reference") (OtherActor :type "Actor Object Reference") (OtherComp :type "PrimitiveComponent Object Reference") (OtherBodyIndex :type Integer) (bFromSweep :type Boolean) (SweepResult :type "HitResult Structure (by ref)"))
  ;[0.1079 0.15 0 0.5] Door Interact
  (`self.EnableInput` (`GameplayStatics.GetPlayerController` 0)))

(event `Key|E`
  (params (Key :type "Key Structure"))
  ;[0.04476 0.15 0 0.5] Open Door
  (:`Pressed`
    (if (`self.bIsOpen`)
      (set `self.bIsOpen` false)
      (else
        (set `self.bIsOpen` true)))))

(event `self.PlayerOverlappDoor.OnComponentEndOverlap`
  (params (OverlappedComponent :type "PrimitiveComponent Object Reference") (OtherActor :type "Actor Object Reference") (OtherComp :type "PrimitiveComponent Object Reference") (OtherBodyIndex :type Integer))
  ;[0.1079 0.15 0 0.5] Door Interact
  (`self.DisableInput` (`GameplayStatics.GetPlayerController` 0) null))

(fn `UserConstructionScript`)