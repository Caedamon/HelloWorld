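; Example Blueprint that demonstrates functions and custom events by printing calculated values to the screen.
; On BeginPlay, a Sequence runs custom events that enable input, print BaseNumber scaled by MultiplyByFactor, and print a DPS figure.
; Pressing A raises BaseNumber and prints the recalculated product.
; Function_CalculateDPS derives DPS from hit damage, fire rate and crit chance.
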(event `self.ReceiveBeginPlay`
  (`|ExecutionSequence`
    (:`then_0`
      (`self.MultiplicationmahDewd`))
    (:`then_1`
      (`self.AdjustBaseNumber` 0))
    (:`then_2`
      (`self.InitializeInput`))
    (:`then_3`
      (`self.DamageDealer`))))

(event `MultiplicationmahDewd`
  ;[0.15 0 0.04535 0.5] Initial Calculation
  (`self.EnableInput` null)
  (bind _result (`self.MultiplyByFactor` 5))
  (`KismetSystemLibrary.PrintString` (`KismetStringLibrary.Conv_IntToString` _result)))

(event `AdjustBaseNumber`
  (params (Adjustment :type Integer))
  ;[0.15 0.04276 0 0.5] Adjust Base
  (set `self.BaseNumber` (+ Adjustment (`self.BaseNumber`)))
  ;[0.15 0.1141 0 0.5] Re‐calculate
  (bind _result (`self.MultiplyByFactor` 5))
  (`KismetSystemLibrary.PrintString` (`KismetStringLibrary.Conv_IntToString` _result)))

(event `InitializeInput`
  ;[0 0.15 0.09176 0.5] Input Handling
  (`self.EnableInput` (`GameplayStatics.GetPlayerController` 0)))

(event `Key|A`
  (params (Key :type "Key Structure"))
  ;[0 0.15 0.09176 0.5] Input Handling
  (:`Pressed`
    (`self.AdjustBaseNumber` 5)))

(event `DamageDealer`
  ;[0 0.1292 0.15 0.5] DPS Display
  (bind _averagedps (`self.Function_CalculateDPS` 18.0))
  (`KismetSystemLibrary.PrintString` (`KismetStringLibrary.Concat_StrStr` "DPS: " (`KismetStringLibrary.Conv_DoubleToString` _averagedps))))

(fn `Function_CalculateDPS`
  (params (`DamagePerHit,` :type "Float (double-precision)" :default 18.0) (FireRate :type "Float (double-precision)" :default 5.0) (CritChance :type "Float (double-precision)" :default 0.3))
  (returns (AverageDPS :type "Float (double-precision)"))
  ;[0.15 0 0.006092 0.5] Calculate DPS
  (return (* (* `DamagePerHit,` FireRate) (+ CritChance 1.0))))

(fn `MultiplyByFactor`
  (params (Factor :type Integer))
  (returns (Result :type Integer))
  ;[0 0.002581 0.15 0.5] Multiply Base by Factor
  (return (* Factor (`self.BaseNumber`))))

(fn `UserConstructionScript`)