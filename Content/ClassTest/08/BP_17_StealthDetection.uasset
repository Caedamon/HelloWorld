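; BP_17_StealthDetection is a test stealth Blueprint that treats any WASD movement as the player being detected.
; Key presses and releases maintain a held-key count and direction flags, from which Tick derives moving and detected states.
; While detected with keys held, it prints an alert and, after HideDelay, reports hiding and clears detection, which Tick recomputes each frame.
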(event `Key|W`
  (params (Key :type "Key Structure"))
  ;[1 0 0 0.5] Movment Keysd
  (:`Pressed`
    (`KismetSystemLibrary.PrintString` "Moving Up")
    (bind _result (`/Engine/EditorBlueprintResources/StandardMacros.IncrementInt` (`self.MovementKeyCount`))
      (:`  `
        (set `self.MovementKeyCount` _result)
        (set `self.bUp` true)
        (`self.Moving`))))
  (:`Released`
    (bind _result_2 (`/Engine/EditorBlueprintResources/StandardMacros.DecrementInt` (`self.MovementKeyCount`))
      (:`  `
        (set `self.MovementKeyCount` _result_2)
        (set `self.bUp` false)))))

(event `Moving`
  ;[1 0 0 0.5] Movment Keysd
  (if (> (`self.MovementKeyCount`) 0)
    (set `self.bPlayerMoving` true)
    (else
      (set `self.bPlayerMoving` false))))

(event `Key|A`
  (params (Key :type "Key Structure"))
  ;[1 0 0 0.5] Movment Keysd
  (:`Pressed`
    (`KismetSystemLibrary.PrintString` "Moving Left")
    (bind _result (`/Engine/EditorBlueprintResources/StandardMacros.IncrementInt` (`self.MovementKeyCount`))
      (:`  `
        (set `self.MovementKeyCount` _result)
        (set `self.bLeft` true)
        (`self.Moving`))))
  (:`Released`
    (bind _result_2 (`/Engine/EditorBlueprintResources/StandardMacros.DecrementInt` (`self.MovementKeyCount`))
      (:`  `
        (set `self.MovementKeyCount` _result_2)
        (set `self.bLeft` false)))))

(event `self.ReceiveBeginPlay`
  (`self.EnableInput` (`GameplayStatics.GetPlayerController` 0))
  (set `self.MovementKeyCount` 0)
  (set `self.bPlayerMoving` false))

(event `Key|S`
  (params (Key :type "Key Structure"))
  ;[1 0 0 0.5] Movment Keysd
  (:`Pressed`
    (`KismetSystemLibrary.PrintString` "Moving Down")
    (bind _result (`/Engine/EditorBlueprintResources/StandardMacros.IncrementInt` (`self.MovementKeyCount`))
      (:`  `
        (set `self.MovementKeyCount` _result)
        (set `self.bDown` true)
        (`self.Moving`))))
  (:`Released`
    (bind _result_2 (`/Engine/EditorBlueprintResources/StandardMacros.DecrementInt` (`self.MovementKeyCount`))
      (:`  `
        (set `self.MovementKeyCount` _result_2)
        (set `self.bDown` false)))))

(event `Key|D`
  (params (Key :type "Key Structure"))
  ;[1 0 0 0.5] Movment Keysd
  (:`Pressed`
    (`KismetSystemLibrary.PrintString` "Moving Right")
    (bind _result (`/Engine/EditorBlueprintResources/StandardMacros.IncrementInt` (`self.MovementKeyCount`))
      (:`  `
        (set `self.MovementKeyCount` _result)
        (set `self.bRight` true)
        (`self.Moving`))))
  (:`Released`
    (bind _result_2 (`/Engine/EditorBlueprintResources/StandardMacros.DecrementInt` (`self.MovementKeyCount`))
      (:`  `
        (set `self.MovementKeyCount` _result_2)
        (set `self.bRight` false)))))

(event `self.ReceiveTick`
  (params (DeltaSeconds :type "Float (single-precision)"))
  (`self.Moving`)
  (`self.IsDetected`)
  (`self.HidingStart`))

(event `IsDetected`
  ;[0.15 0 0.03893 0.5] IsDetected?
  (if (`self.bPlayerMoving`)
    (set `self.bPlayerDetected` true)
    (else
      (set `self.bPlayerDetected` false))))

(event `HidingStart`
  ; Comment
  (if (`self.bPlayerDetected`)
    (`KismetSystemLibrary.PrintString` "Player Detected!" true true (struct :`G` 0.66 :`B` 1.0 :`A` 1.0) (`GameplayStatics.GetWorldDeltaSeconds`))
    (if (> (`self.MovementKeyCount`) 0)
      (`KismetSystemLibrary.Delay` (`self.HideDelay`))
      (`KismetSystemLibrary.PrintString` "Player in Hiding")
      (set `self.bPlayerDetected` false))))

(fn `UserConstructionScript`)