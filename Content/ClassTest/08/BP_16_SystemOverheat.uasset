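; BP_16_SystemOverheat is a test Blueprint that simulates a system heating and cooling against overheat and cool thresholds, reporting through printed messages.
; Each Tick calls TempGuage, which zeroes Temperature on both branches before re-evaluating IsCooling.
; Tick then runs Heating when IsCooling is true, otherwise Cooling, so the flag reads inverted.
; Both adjust Temperature by a delta-time-scaled rate and set IsCooling past their threshold.
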(event `Heating`
  ;[0.15 0.005636 0 0.5] IsHeating
  (set `self.Temperature` (+ (`self.Temperature`) (* (`self.HeatRate`) (`GameplayStatics.GetWorldDeltaSeconds`))))
  (if (> (`self.Temperature`) (`self.OverheatThreshold`))
    (`KismetSystemLibrary.PrintString` "System Heated Up!")
    (set `self.bIsCooling` true)))

(event `Cooling`
  ;[0 0.0322 0.15 0.5] IsCooling
  (set `self.Temperature` (- (`self.Temperature`) (* (`self.CoolRate`) (`GameplayStatics.GetWorldDeltaSeconds`))))
  (if (< (`self.Temperature`) (`self.CoolThreshold`))
    (`KismetSystemLibrary.PrintString` "System cooled down.")
    (set `self.bIsCooling` false)))

(event `self.ReceiveTick`
  (params (DeltaSeconds :type "Float (single-precision)"))
  ;[0.15 0 0.07505 0.5] ActiveTemperatureCheck
  (`self.TempGuage`)
  (if (`self.bIsCooling`)
    (`KismetSystemLibrary.PrintString` "System is Heating up!" true true (struct :`G` 0.66 :`B` 1.0 :`A` 1.0) (`GameplayStatics.GetWorldDeltaSeconds`))
    (`self.Heating`)
    (else
      (`KismetSystemLibrary.PrintString` "System is Cooling Down!" true true (struct :`G` 0.66 :`B` 1.0 :`A` 1.0) (`GameplayStatics.GetWorldDeltaSeconds`))
      (`self.Cooling`))))

(event `TempGuage`
  ;[0 0.15 0.134 0.5] Temp Checker
  (if (or (>= (`self.Temperature`) (`self.OverheatThreshold`)) (<= (`self.Temperature`) (`self.CoolThreshold`)))
    (bind _output_get (set `self.Temperature` 0.0))
    (set `self.bIsCooling` (and (>= _output_get (`self.OverheatThreshold`)) (not (`self.bIsCooling`))))
    (`KismetSystemLibrary.PrintString` "System Overheated!")
    (else
      (bind _output_get_2 (set `self.Temperature` 0.0))
      (set `self.bIsCooling` (and (<= _output_get_2 (`self.CoolThreshold`)) (`self.bIsCooling`)))
      (`KismetSystemLibrary.PrintString` "System Cooling Down!"))))

(fn `UserConstructionScript`)