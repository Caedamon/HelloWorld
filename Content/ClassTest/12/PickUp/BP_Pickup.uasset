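; BP_Pickup is a pickup actor with an empty Pickup function, apparently a base for specific pickups to override.
; When the player 0 pawn begins overlapping its Collision component, it calls Pickup and destroys itself.
; On BeginPlay, a timeline animates CenterPoint's relative height, scaled by CoinAnimHeight, and its yaw.
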(event `self.Collision.OnComponentBeginOverlap`
  (params (OverlappedComponent :type "PrimitiveComponent Object Reference") (OtherActor :type "Actor Object Reference") (OtherComp :type "PrimitiveComponent Object Reference") (OtherBodyIndex :type Integer) (bFromSweep :type Boolean) (SweepResult :type "HitResult Structure (by ref)"))
  ;[0.15 0 0.04743 0.5] Overlap
  (if (== OtherActor (`GameplayStatics.GetPlayerPawn` 0))
    (`self.Pickup`)
    (`self.K2_DestroyActor`)))

(event `self.ReceiveBeginPlay`
  ;[0.15 0.003551 0 0.5] Z and X lvl Animations
  (bind (_direction _height _rotation) (`Timeline|Timeline` :!via `PlayFromStart`)
    (:`Update`
      (`SceneComponent.K2_SetRelativeTransform` (`self.CenterPoint`) (`KismetMathLibrary.MakeTransform` (`KismetMathLibrary.MakeVector` 0.0 0.0 (* _height (`self.CoinAnimHeight`))) (`KismetMathLibrary.MakeRotator` 0.0 0.0 (.z _rotation))) false false))))

(fn `Pickup`)

(fn `UserConstructionScript`)