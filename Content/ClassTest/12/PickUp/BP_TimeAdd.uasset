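; BP_TimeAdd is a pickup that adds bonus time to the level's countdown when collected.
; It overrides Pickup, runs the parent behavior, then casts the game mode to BP_CubeGameMode and increases TimeLeft by its TimeBonus variable.
; The event graph holds only disabled placeholder nodes, and the construction script just calls the parent.
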(fn `Pickup`
  (`parent.Pickup`)
  (bind _asbp_cube_game_mode (cast `/Game/ClassTest/11/System/BP_CubeGameMode` (`GameplayStatics.GetGameMode`)))
  (set `/Game/ClassTest/11/System/BP_CubeGameMode.TimeLeft` (+ (`/Game/ClassTest/11/System/BP_CubeGameMode.TimeLeft` _asbp_cube_game_mode) (`self.TimeBonus`)) _asbp_cube_game_mode))

(fn `UserConstructionScript`
  (`parent.UserConstructionScript`))