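; BP_10_LogicalOperators is a test Blueprint that exercises boolean AND, OR and NOT logic on speed, scale and sum variables.
; BeginPlay uses a Sequence to call five custom events in order.
; Each event combines comparisons into one Branch condition, from simple pairs to nested expressions, and prints a pass or fail message.
; The graph only reads its variables, and the construction script is empty.
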(event `CustomEvent_CheckSpeedAndScale`
  ;[0.15 0 0.04261 0.5] UNLEASH THE KRAKEN! Speed Check
  (if (and (< (`self.NewSpeed`) (`self.SpeedThreshold`)) (and (<= (`self.ScaleFactor`) (`self.MinScale`)) (>= (`self.ScaleFactor`) (`self.MaxScale`))))
    (`KismetSystemLibrary.PrintString` "Speed is low and scale factor is acceptable")
    (else
      (`KismetSystemLibrary.PrintString` "Conditions not met! UNLEASH THE KRAKEN!"))))

(event `self.ReceiveBeginPlay`
  ;[0 0.09581 0.15 0.5] ITS A KRAKKEN!
  (`|ExecutionSequence`
    (:`then_0`
      (`self.CustomEvent_CheckSpeedAndScale`))
    (:`then_1`
      (`self.CustomEvent_ValidateSpeedOrScale`))
    (:`then_2`
      (`self.CustomEvent_CombinedConditions`))
    (:`then_3`
      (`self.CustomEvent_NegateCondition`))
    (:`then_4`
      (`self.CustomEvent_ComplexLogicalExpression`))))

(event `CustomEvent_ValidateSpeedOrScale`
  ;[0.01455 0 0.15 0.5] Validate Speed
  (if (or (> (`self.AdjustedSpeed`) (`self.InitialSpeed`)) (< (`self.ScaleFactor_2`) (`self.ScaleThreshold`)))
    (`KismetSystemLibrary.PrintString` "Either adjusted speed is higher or scale \nfactor is above 1.5")
    (else
      (`KismetSystemLibrary.PrintString` "Neither condition is met"))))

(event `CustomEvent_CombinedConditions`
  ;[0.15 0 0.003836 0.5] Devestators Ready for Annihilation!
  (if (and (> (`self.Sum`) (`self.FinalValue`)) (>= (`self.NewSpeed_2`) (`self.MinSafeSpeed`)))
    (`KismetSystemLibrary.PrintString` "Sum is greater and speed is safe")
    (else
      (`KismetSystemLibrary.PrintString` "Conditions NOT met! PREPARE THE DEVESTATORS!"))))

(event `CustomEvent_NegateCondition`
  ;[0 0.15 0.08815 0.5] What do you mean "comment"???
  (if (not (and (>= (`self.ScaleFactor_3`) (`self.MinScale_2`)) (<= (`self.ScaleFactor_3`) (`self.MaxScale_2`))))
    (`KismetSystemLibrary.PrintString` "Scale factor is not within the acceptable \nrange.")
    (else
      (`KismetSystemLibrary.PrintString` "Scale factor is acceptable."))))

(event `CustomEvent_ComplexLogicalExpression`
  ;[0.1192 0.15 0 0.5] Complex Conditions
  (if (and (or (> (`self.Sum_2`) (`self.FinalValue_2`)) (< (`self.NewSpeed_3`) (`self.SpeedLimit`))) (> (`self.ScaleFactor_4`) (`self.MinScale_3`)))
    (`KismetSystemLibrary.PrintString` "Complex Conditions Met!")
    (else
      (`KismetSystemLibrary.PrintString` "Complex Conditions Not Met!"))))

(fn `UserConstructionScript`)