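; Day/night clock Blueprint that simulates a 24-hour time of day and announces its main phases through debug prints only.
; Each Tick advances TimeOfDay by DeltaSeconds times TimeScale, resets it at 24 and prints the running time.
; Tick then runs sunrise, midday, sunset and midnight checks against narrow hour windows.
; LastPhase prevents repeat triggers within a window, so each phase change prints its name once.
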(event `self.ReceiveTick`
  (params (DeltaSeconds :type "Float (single-precision)"))
  ;[0 0.15 0.003905 0.5] Make sure each "time of day" checks with tick.
  (`self.Clock `)
  (`|ExecutionSequence`
    (:`then_0`
      (`self.Sunrise`))
    (:`then_1`
      (`self.Mid-day`))
    (:`then_2`
      (`self.Sunset`))
    (:`then_3`
      (`self.Midnight`))))

(event `Clock`
  ;[0 0.15 0.03096 0.5] Clock that prints out The hour and .xx minuts.
  (bind _output_get (set `self.TimeOfDay` (+ (* (stale `self.ReceiveTick` DeltaSeconds) (`self.TimeScale`)) (`self.TimeOfDay`))))
  (if (>= _output_get 24.0)
    (set `self.TimeOfDay` 0.0)
    (else
      (`KismetSystemLibrary.PrintString` (`KismetStringLibrary.Concat_StrStr` "Time: " (`KismetTextLibrary.Conv_TextToString` (`KismetTextLibrary.Conv_DoubleToText` (`self.TimeOfDay`) "HalfToEven" false true 1 324 2 2))) true true (struct :`G` 0.66 :`B` 1.0 :`A` 1.0) (`GameplayStatics.GetWorldDeltaSeconds`)))))

(event `Sunrise`
  ;[0.15 0.05373 0.1111 0.5] Sunrise Checker
  (if (and (`KismetMathLibrary.InRange_FloatFloat` (`self.TimeOfDay`) 5.9 6.1) (!= "Sunrise" (`self.LastPhase`)))
    (set `self.LastPhase` "Sunrise")
    (`self.PrintTimeOfDay`)))

(event `Sunset`
  ;[0.15 0.002808 0 0.5] Sunset Checker
  (if (and (`KismetMathLibrary.InRange_FloatFloat` (`self.TimeOfDay`) 17.9 18.1) (!= "Sunset" (`self.LastPhase`)))
    (set `self.LastPhase` "Sunset")
    (`self.PrintTimeOfDay`)))

(event `Mid-day`
  ;[0.15 0.08942 0 0.5] Mid-day Checker
  (if (and (`KismetMathLibrary.InRange_FloatFloat` (`self.TimeOfDay`) 11.9 12.1) (!= "Mid-day" (`self.LastPhase`)))
    (set `self.LastPhase` "Mid-day")
    (`self.PrintTimeOfDay`)))

(event `Midnight`
  ;[0 0 0 0.5] Midnight Checker
  (if (and (or (`KismetMathLibrary.InRange_FloatFloat` (`self.TimeOfDay`) 23.9 24.0) (`KismetMathLibrary.InRange_FloatFloat` (`self.TimeOfDay`) 0.0 0.1)) (!= "Midnight" (`self.LastPhase`)))
    (set `self.LastPhase` "Midnight")
    (`self.PrintTimeOfDay`)))

(fn `PrintTimeOfDay`
  (`KismetSystemLibrary.PrintString` (`self.LastPhase`)))

(fn `UserConstructionScript`)