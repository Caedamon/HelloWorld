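; BP_9_ThreatDetectors is a class-exercise Blueprint that runs threshold checks on health, ammo, time and score and prints status messages.
; BeginPlay uses a Sequence to call four custom events in order.
; Each event makes one comparison on its variables, such as a health ratio or a clip-full test, and branches to a pass or fail Print String.
; Checks run once at start, and the construction script is empty.
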(event `CustomEvent_LowHealthAlert`
  ;[0.7188 0.4026 0.0882 0.5] Health Checker
  (bind _output_get (set `self.HealthRatio` (/ (`self.CurrentHealth`) (`self.MaxHealth`))))
  (if (< _output_get 0.25)
    (`KismetSystemLibrary.PrintString` "Warning! Critical health!")
    (else
      (`KismetSystemLibrary.PrintString` "Health is OK!"))))

(event `self.ReceiveBeginPlay`
  ;[0.09693 0 0.15 0.5] Chandeler setup is awesome!
  (`|ExecutionSequence`
    (:`then_0`
      (`self.CustomEvent_LowHealthAlert`))
    (:`then_1`
      (`self.CustomEvent_CheckAmmo`))
    (:`then_2`
      (`self.CustomEvent_TimeGate`))
    (:`then_3`
      (`self.CustomEvent_CheckHighScore`))))

(event `CustomEvent_CheckAmmo`
  ;[0 0.1395 0.15 0.5] Comment
  (if (== (`self.CurrentAmmo`) (`self.ClipSize`))
    (`KismetSystemLibrary.PrintString` "The Clip is Fully Loaded!")
    (else
      (`KismetSystemLibrary.PrintString` "A Reload is Possible!"))))

(event `CustomEvent_TimeGate`
  ;[0.05377 0.05762 0.15 0.5] Gate Timer!
  (if (>= (`self.ElapsedTime`) (`self.TargetTime`))
    (`KismetSystemLibrary.PrintString` "You are to late adventurer! the gates closed!")
    (else
      (`KismetSystemLibrary.PrintString` "Great timing! your just in time, Gates still open!"))))

(event `CustomEvent_CheckHighScore`
  ;[0 0.15 0.0086 0.5] Score Checker
  (if (>= (`self.Score`) (`self.HighScoreThreshold`))
    (`KismetSystemLibrary.PrintString` "NEW HIGHSCORE! CONGRATS!")
    (else
      (`KismetSystemLibrary.PrintString` "Eeehhh, you coulda done better looser!" true true (struct :`R` 1.0 :`G` 0.085289 :`A` 1.0)))))

(fn `UserConstructionScript`)