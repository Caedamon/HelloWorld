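; BP_14_SpeedMod is a test Blueprint that simulates a speed value rising and decaying with Left Shift input.
; BeginPlay enables player input, and holding or releasing Left Shift toggles IsAccelerating.
; Tick prints CurrentSpeed and adjusts it by Acceleration or DecayRate scaled by delta time.
; Clamping only triggers the max and base speed messages; CurrentSpeed itself stays unclamped and drives no movement.
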(event `self.ReceiveTick`
  (params (DeltaSeconds :type "Float (single-precision)"))
  (`|ExecutionSequence`
    (:`then_0`
      ;[0 0.15 0.03096 0.5] Speed Printer
      (`KismetSystemLibrary.PrintString` (`KismetStringLibrary.Conv_DoubleToString` (`self.CurrentSpeed`)) true true (struct :`G` 0.66 :`B` 1.0 :`A` 1.0) (`GameplayStatics.GetWorldDeltaSeconds`)))
    (:`then_1`
      (if (`self.bIsAccelerating`)
        ;[0.15 0 0.007236 0.5] Set Accelleration
        (bind _output_get (set `self.CurrentSpeed` (+ (`self.CurrentSpeed`) (* (`self.Acceleration`) (`GameplayStatics.GetWorldDeltaSeconds`)))))
        (`KismetSystemLibrary.PrintString` "MAX SPEED REACHED!" (== (`KismetMathLibrary.FClamp` _output_get (`self.BaseSpeed`) (`self.MaxSpeed`)) (`self.MaxSpeed`)) true (struct :`R` 1.0 :`B` 0.076232 :`A` 1.0) (`GameplayStatics.GetWorldDeltaSeconds`))
        (else
          ;[0.15 0 0.101 0.5] Set Decelleration
          (bind _output_get_2 (set `self.CurrentSpeed` (- (`self.CurrentSpeed`) (* (`self.DecayRate`) (`GameplayStatics.GetWorldDeltaSeconds`)))))
          (`KismetSystemLibrary.PrintString` "Base Speed Attained" (== (`KismetMathLibrary.FClamp` _output_get_2 (`self.BaseSpeed`) (`self.MaxSpeed`)) (`self.BaseSpeed`)) true (struct :`G` 1.0 :`B` 0.114498 :`A` 1.0) (`GameplayStatics.GetWorldDeltaSeconds`)))))))

(event `Key|LeftShift`
  (params (Key :type "Key Structure"))
  ;[0 0.01605 0.15 0.5] Controller
  (:`Pressed`
    (if true
      (set `self.bIsAccelerating` true)
      (`KismetSystemLibrary.PrintString` "Starting Accelerating")))
  (:`Released`
    (if true
      (set `self.bIsAccelerating` false)
      (`KismetSystemLibrary.PrintString` "Starting Deceleration"))))

(event `self.ReceiveBeginPlay`
  ;[0 0.01605 0.15 0.5] Controller
  (`self.EnableInput` (`GameplayStatics.GetPlayerController` 0)))

(fn `UserConstructionScript`)